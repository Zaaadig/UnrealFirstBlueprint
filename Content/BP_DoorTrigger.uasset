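; Trigger actor that alternately opens and closes a referenced door each time the player enters its box.
; The construction script gives the Base mesh a dynamic material instance tinted with a starting color.
; On overlap by an actor tagged Player, it switches that tint to a second color, never reverted, and a FlipFlop alternates the open and close calls on DoorREF.
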(event OnComponentBeginOverlap(Box)
  (params (OverlappedComponent :type Primitive%20Component%20Object%20Reference) (OtherActor :type Actor%20Object%20Reference) (OtherComp :type Primitive%20Component%20Object%20Reference) (OtherBodyIndex :type Integer) (bFromSweep :type Boolean) (SweepResult :type Hit%20Result%20Structure%20%28by%20ref%29))
  (if (Actor|ActorHasTag OtherActor "Player")
    (Rendering|Material|SetVectorParameterValue (Variables|Default|GetDynMat_TriggerBase) "Base Color" (Variables|Default|GetColorV2) :!class /Script/Engine.MaterialInstanceDynamic)
    (Utilities|FlowControl|FlipFlop
      (:A
        (Class|BPITriggers|OuverturePorte(Message) (Variables|Default|GetDoor%20REF)))
      (:B
        (Default|FermeturePorte (Variables|Default|GetDoor%20REF))))))

(event EventBeginPlay)

(event Collision|EventActorBeginOverlap
  (params (OtherActor :type Actor%20Object%20Reference)))

(event EventTick
  (params (DeltaSeconds :type Float%20%28single-precision%29)))

(fn ConstructionScript
  (bind _returnvalue (Rendering|Material|CreateDynamicMaterialInstance (Variables|Default|GetBase) 0 "/Game/MI_Basic_Parameter.MI_Basic_Parameter" "None" :!class /Script/Engine.PrimitiveComponent))
  (bind _output_get (Variables|Default|SetDynMat_TriggerBase _returnvalue))
  (Rendering|Material|SetVectorParameterValue _output_get "Base Color" (Variables|Default|GetColor) :!class /Script/Engine.MaterialInstanceDynamic))