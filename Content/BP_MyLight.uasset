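; BP_MyLight is a configurable light actor with a static mesh and a point light that can optionally pulse.
; The construction script applies mesh scale and the light's intensity, units, color, radius and source shape settings from variables.
; With BlsShinning set, BeginPlay starts a timeline that lerps intensity between zero and LightIntensity.
; A delayed FlipFlop on Finished alternates reverse and forward playback, looping the pulse.
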(event Custom|PlayTimeline
  (bind _alpha (Timeline|TL_ShinningLight PlayFromStart)
    (:Update
      (Rendering|Components|Light|SetIntensity (Variables|Default|GetPointLight) (Math|Float|Lerp 0.0 (Variables|Default|GetLight_Intensity) _alpha)))
    (:Finished
      (Utilities|FlowControl|Delay (Variables|Default|GetShinningDelay))
      (Utilities|FlowControl|FlipFlop
        (:A
          (CallFunction|ReverseTimeline))
        (:B
          (CallFunction|PlayTimeline))))))

(event Custom|Reverse%20Timeline
  (bind _alpha (Timeline|TL_ShinningLight ReverseFromEnd)
    (:Update
      (Rendering|Components|Light|SetIntensity (Variables|Default|GetPointLight) (Math|Float|Lerp 0.0 (Variables|Default|GetLight_Intensity) _alpha)))
    (:Finished
      (Utilities|FlowControl|Delay (Variables|Default|GetShinningDelay))
      (Utilities|FlowControl|FlipFlop
        (:A
          (CallFunction|ReverseTimeline))
        (:B
          (CallFunction|PlayTimeline))))))

(event EventBeginPlay
  (if (Variables|Default|GetblsShinning)
    (Components|Timeline|SetPlayRate (Variables|Default|GetTL_ShinningLight) (/ 1.0 (Variables|Default|GetTL_ShinningLight_Rate)))
    (CallFunction|PlayTimeline)))

(event Collision|EventActorBeginOverlap
  (params (OtherActor :type Actor%20Object%20Reference)))

(event EventTick
  (params (DeltaSeconds :type Float%20%28single-precision%29)))

(fn ConstructionScript
  (Utilities|FlowControl|Sequence
    (:then_0
      (Transformation|SetWorldScale3D (Variables|Default|GetStaticMesh) (Math|Conversions|ToVector(Float) (Variables|Default|GetScale))))
    (:then_1
      (Rendering|Components|Light|SetIntensity (Variables|Default|GetPointLight) (Variables|Default|GetLight_Intensity))
      (Class|LocalLightComponent|SetIntensityUnits (Variables|Default|GetPointLight) (Variables|Default|GetLight_IntensityUnits))
      (Rendering|Components|Light|SetLightColor (Variables|Default|GetPointLight) (Math|Conversions|ToLinearColor(Color) (Variables|Default|GetLight_Color)) true))
    (:then_2
      (Rendering|Lighting|SetAttenuationRadius (Variables|Default|GetPointLight) (Variables|Default|GetLight_AttenuationRadius))
      (Class|PointLightComponent|SetSourceRadius (Variables|Default|GetPointLight) (Variables|Default|GetLight_SourceRadius))
      (Class|PointLightComponent|SetSoftSourceRadius (Variables|Default|GetPointLight) (Variables|Default|GetLight_SoftSourceRadius))
      (Class|PointLightComponent|SetSourceLength (Variables|Default|GetPointLight) (Variables|Default|GetLight_SourceLenght)))))