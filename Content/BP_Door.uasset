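; BP_Door is a colored door that slides vertically when its open and close events are called.
; A Timeline lerps the door mesh's relative location toward the FinalLocation height, with play rate set from TLOpenRate as a duration, and reverses to close.
; The construction script creates a dynamic material tinted with the Color variable; opening turns it black, and closing does not restore it.
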(event Custom|CloseDoor
  (bind _alpha (Timeline|Timeline Reverse)
    (:Update
      (Transformation|SetRelativeLocation (Variables|Default|GetSM_Door) (Math|Vector|Lerp(Vector) "0.000000,0.000000,70.000000" (Math|Vector|MakeVector 0.0 0.0 (Variables|Default|GetFinal%20Location)) _alpha) false false))))

(event Custom|Fermeture%20porte_1
  (Components|Timeline|SetPlayRate (Variables|Default|GetTimeline) (/ 1.0 (Variables|Default|GetTL_Open_Rate)))
  (CallFunction|CloseDoor))

(event EventBeginPlay)

(event Collision|EventActorBeginOverlap
  (params (OtherActor :type Actor%20Object%20Reference)))

(event EventTick
  (params (DeltaSeconds :type Float%20%28single-precision%29)))

(event EventOuverturePorte
  (Rendering|Material|SetVectorParameterValue :self (Variables|Default|GetDynMat_TriggerDoor) :ParameterName "Base Color" :!class /Script/Engine.MaterialInstanceDynamic)
  (Components|Timeline|SetPlayRate (Variables|Default|GetTimeline) (/ 1.0 (Variables|Default|GetTL_Open_Rate)))
  (bind _alpha (Timeline|Timeline Play)
    (:Update
      (Transformation|SetRelativeLocation (Variables|Default|GetSM_Door) (Math|Vector|Lerp(Vector) "0.000000,0.000000,70.000000" (Math|Vector|MakeVector 0.0 0.0 (Variables|Default|GetFinal%20Location)) _alpha) false false))))

(fn ConstructionScript
  (bind _returnvalue (Rendering|Material|CreateDynamicMaterialInstance (Variables|Default|GetSM_Door) 0 "/Game/MI_Basic_Parameter.MI_Basic_Parameter" "None" :!class /Script/Engine.PrimitiveComponent))
  (bind _output_get (Variables|Default|SetDynMat_TriggerDoor _returnvalue))
  (Rendering|Material|SetVectorParameterValue _output_get "Base Color" (Variables|Default|GetColor) :!class /Script/Engine.MaterialInstanceDynamic))